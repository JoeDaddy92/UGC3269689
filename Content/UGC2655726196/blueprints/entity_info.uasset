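; An entity info Blueprint that shows the display names of actors overlapping it on a text render, or "Place Entity Here" when empty.
; Begin and end overlap events add or remove actors in a set, then rebuild the text from it.
; An optional whitelist admits only classes named like guns, grenades or knives, excluding Tasers, by substring matching.
; A Clear function empties the set and resets the text.
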(event `self.ReceiveActorBeginOverlap`
  (params (OtherActor :type "Actor Object Reference"))
  (bind _passthrough (`self.WhiteListMacro` OtherActor)
    (:`CandidatePassed`
      (`BlueprintSetLibrary.Set_Add` (`self.ActorRefs`) _passthrough)
      (`self.UpdateText`))))

(event `self.ReceiveActorEndOverlap`
  (params (OtherActor :type "Actor Object Reference"))
  (bind _passthrough (`self.WhiteListMacro` OtherActor)
    (:`CandidatePassed`
      (`BlueprintSetLibrary.Set_Remove` (`self.ActorRefs`) _passthrough)
      (`self.UpdateText`))))

(fn `CheckWhiteList`
  (params (actor :type "Actor Object Reference"))
  (returns (passed :type Boolean))
  (bind _returnvalue (`KismetSystemLibrary.GetClassDisplayName` (`GameplayStatics.GetObjectClass` actor)))
  (return (and (or (`KismetStringLibrary.Contains` _returnvalue "Gun") (`KismetStringLibrary.Contains` _returnvalue "Grenade") (`KismetStringLibrary.Contains` _returnvalue "Knife")) (not (`KismetStringLibrary.Contains` _returnvalue "Taser")))))

(fn `Clear`
  (`BlueprintSetLibrary.Set_Clear` (`self.ActorRefs`))
  (`self.UpdateText`))

(fn `UpdateText`
  (locals (buffer :type String))
  (set `local.buffer` "")
  (bind _result (`BlueprintSetLibrary.Set_ToArray` (`self.ActorRefs`)))
  (if (> (`KismetArrayLibrary.Array_Length` _result) 0)
    (for _array_element _result
      (set `local.buffer` (`KismetStringLibrary.Concat_StrStr` (`KismetSystemLibrary.GetDisplayName` _array_element) " \n" (`local.buffer`))))
    (`TextRenderComponent.K2_SetText` (`self.TextRender`) (`KismetTextLibrary.Conv_StringToText` (`local.buffer`)))
    (else
      (`TextRenderComponent.K2_SetText` (`self.TextRender`) "Place Entity Here"))))

(fn `UserConstructionScript`)