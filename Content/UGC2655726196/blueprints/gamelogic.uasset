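; Game logic Blueprint for a Pavlov custom map that removes the stock Team Deathmatch game mode one second after BeginPlay.
; It finds that actor by scanning all actors for a matching class display name, then destroys it.
; An unconnected chain would set up a no-team respawn mode with unlimited-style buying and cash.
; Debug helpers report player status and actor classes through PlayerModifier and server messages, gated by a setting.
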(event `self.ReceiveBeginPlay`
  (`KismetSystemLibrary.Delay` 1.0)
  (bind _actors (`self.findAllActorsWithClassName` "TeamDeathMatchGameMode_C"))
  (for _array_element _actors
    (`self.K2_DestroyActor` _array_element)))

(fn `findAllActorsWithClassName`
  (params (className :type String))
  (returns (actors :type "Array of Actor Object Reference"))
  (locals (tmp :type "Array of Actor Object Reference"))
  (bind _tmp (`local.tmp`))
  (bind _outactors (`GameplayStatics.GetAllActorsOfClass` "/Script/Engine.Actor"))
  (for _array_element _outactors
    (if (`KismetStringLibrary.EqualEqual_StrStr` (`KismetSystemLibrary.GetClassDisplayName` (`GameplayStatics.GetObjectClass` _array_element)) className)
      (`KismetArrayLibrary.Array_Append` _tmp (`|MakeArray` _array_element))))
  (return _tmp))

(fn `print`
  (params (line :type String))
  (`/UGC3269689/UGC2655726196/blueprints/modifiers/player_modifier.print` (`self.playerModifier`) line)
  (`Pavlov_Library.SendAllMsg` (make `Message` "Server" (`KismetTextLibrary.Conv_StringToText` line))))

(fn `printAllActorClasses`
  (locals (uniqueNames :type "Set of String"))
  (bind _outactors (`GameplayStatics.GetAllActorsOfClass` "/Script/Engine.Actor"))
  (for _array_element _outactors
    (`BlueprintSetLibrary.Set_Add` (`local.uniqueNames`) (`KismetSystemLibrary.GetClassDisplayName` (`GameplayStatics.GetObjectClass` _array_element))))
  (bind _result (`BlueprintSetLibrary.Set_ToArray` (`local.uniqueNames`)))
  (for _array_element_2 _result
    (`self.printDebug` _array_element_2)))

(fn `printDebug`
  (params (line :type String))
  (if (`BlueprintMapLibrary.Map_Find` (`self.boolSettings`) "NewEnumerator4")
    (`self.print` line)))

(fn `printPlayerState`
  (params (pawn :type "Pawn Object Reference"))
  (bind _playerstatus (`PavlovProxyStatics.GetPavlovPlayerStatusByPawn` pawn))
  (`self.printDebug` (`KismetStringLibrary.Concat_StrStr` "" "; \n  Dead Time: " (`KismetStringLibrary.Conv_DoubleToString` (`.DeadTime` (break `PavlovPlayerStatus` _playerstatus))) "; Alive Time: " (`KismetStringLibrary.Conv_DoubleToString` (`.AliveTime` (break `PavlovPlayerStatus` _playerstatus))))))

(fn `UserConstructionScript`)