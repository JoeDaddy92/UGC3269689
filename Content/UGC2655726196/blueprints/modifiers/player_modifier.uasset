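; Player modifier that registers itself with the game logic on construction and drives a temporary on-screen message console.
; Print appends a line to a buffer and spawns a Console_print_delay actor holding a reference back to the modifier.
; ClearLine removes the oldest line, presumably called by that delay actor.
; Both refresh the Console text by joining the buffer with each later line prepended, so the newest appears first.
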(fn `_clearLine`
  (`KismetArrayLibrary.Array_Remove` (`self.console_buffer`))
  (`self._updateDisplay`))

(fn `_updateDisplay`
  (locals (buffer :type String))
  (for _array_element (`self.console_buffer`)
    (set `local.buffer` (`KismetStringLibrary.Concat_StrStr` _array_element " \n" (`local.buffer`))))
  (`TextRenderComponent.K2_SetText` (`self.Console`) (`KismetTextLibrary.Conv_StringToText` (`local.buffer`))))

(fn `print`
  (params (line :type String))
  (`KismetArrayLibrary.Array_Append` (`self.console_buffer`) (`|MakeArray` line))
  (`self._updateDisplay`)
  (`|SpawnActorFromClass` "/UGC3269689/UGC2655726196/blueprints/modifiers/console_print_delay.console_print_delay_C" (`KismetMathLibrary.MakeTransform` (0.0 0.0 0.0)) "Undefined" "OverrideRootScale" null self null))

(fn `UserConstructionScript`
  (bind _gamelogic (`/UGC3269689/UGC2655726196/blueprints/ActorMacros.GetGameLogic`)
    (:`ExecOut`
      (set `/UGC3269689/UGC2655726196/blueprints/gamelogic.playerModifier` self _gamelogic))))