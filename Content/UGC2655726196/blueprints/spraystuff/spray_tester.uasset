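; Spray tester target actor that records weapon hit patterns from point damage.
; Each hit is converted to an offset from the actor with X and Y swapped, then sent to a Button reference with the time since the previous hit and the damage causer's name.
; The unswapped offset and interval are also printed and shown on PosText.
; A bullet speed readout is present but never runs.
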(event `self.ReceivePointDamage`
  (params (Damage :type "Float (single-precision)") (DamageType :type "DamageType Object Reference") (HitLocation :type "Vector Structure") (HitNormal :type "Vector Structure") (HitComponent :type "PrimitiveComponent Object Reference") (BoneName :type Name) (ShotFromDirection :type "Vector Structure") (InstigatedBy :type "Controller Object Reference") (DamageCauser :type "Actor Object Reference") (HitInfo :type "HitResult Structure (by ref)"))
  (bind _returnvalue (- HitLocation (`self.K2_GetActorLocation`)))
  (bind _time_elapsed (`self.getTimeElapsed`))
  (`/UGC3269689/UGC2655726196/blueprints/spraystuff/save_button.addDataPoint` (`self.button`) (`KismetMathLibrary.MakeVector` (.y _returnvalue) (.x _returnvalue) (.z _returnvalue)) _time_elapsed (`KismetSystemLibrary.GetObjectName` DamageCauser))
  (bind _returnvalue_2 (`KismetStringLibrary.Concat_StrStr` (`KismetStringLibrary.Conv_VectorToString` _returnvalue) "; " (`KismetStringLibrary.Conv_DoubleToString` _time_elapsed)))
  (`KismetSystemLibrary.PrintString` _returnvalue_2)
  (`TextRenderComponent.K2_SetText` (`self.PosText`) (`KismetTextLibrary.Conv_StringToText` _returnvalue_2)))

(fn `getTimeElapsed`
  (returns (time_elapsed :type "Float (double-precision)"))
  (locals (elapsed :type "Float (double-precision)") (newLastTime :type "Float (double-precision)"))
  (bind _output_get (set `local.newLastTime` (`GameplayStatics.GetRealTimeSeconds`)))
  (set `local.elapsed` (- _output_get (`self.last_time`)))
  (set `self.last_time` _output_get)
  (return (`local.elapsed`)))

(fn `UserConstructionScript`
  (set `self.last_time` (`GameplayStatics.GetRealTimeSeconds`)))