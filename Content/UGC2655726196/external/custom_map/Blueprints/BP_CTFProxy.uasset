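; BP_CTFProxy is a short-lived capture-the-flag marker for a custom map, carrying flag settings as actor tags.
; The construction script rebuilds the tags from scratch: a flag identifier, the owning team ID, the return time and an optional no-flag marker.
; Values are encoded into tag names by string concatenation, so they can be read without referencing this class.
; On BeginPlay it sets a 20-second lifespan.
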(event `self.ReceiveBeginPlay`
  (`self.SetLifeSpan` 20.0))

(fn `UserConstructionScript`
  (bind _tags (`self.Tags`))
  (`KismetArrayLibrary.Array_Clear` _tags)
  (`KismetArrayLibrary.Array_AddUnique` _tags "ctfflag")
  (`KismetArrayLibrary.Array_AddUnique` _tags (`KismetStringLibrary.Conv_StringToName` (`KismetStringLibrary.Concat_StrStr` "team" (`KismetStringLibrary.Conv_IntToString` (`self.OwningTeamID`)))))
  (`KismetArrayLibrary.Array_AddUnique` _tags (`KismetStringLibrary.Conv_StringToName` (`KismetStringLibrary.Concat_StrStr` "ReturnTime" (`KismetStringLibrary.Conv_IntToString` (`self.ReturnTime`)))))
  (if (`self.NoFlag?`)
    (`KismetArrayLibrary.Array_AddUnique` _tags "NoFlag")))