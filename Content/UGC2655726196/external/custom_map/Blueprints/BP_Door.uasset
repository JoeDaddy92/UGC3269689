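; Automatic door for a Pavlov custom map that opens when a player pawn enters its trigger box and closes once no characters remain inside.
; Overlap events set the rep-notify Open variable, whose OnRep plays or reverses the MoveDoor timeline to keep the door synced.
; The timeline lerps between closed and open transforms, applying rotation or location per RotateOpen, which also toggles the construction-script arrow.
; Round start resets the door to closed.
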(event `/CustomMapTools/Blueprints/BPI_MatchRounds.RoundStarting`
  (set `self.Open?` false))

(event `self.Box.OnComponentBeginOverlap`
  (params (OverlappedComponent :type "PrimitiveComponent Object Reference") (OtherActor :type "Actor Object Reference") (OtherComp :type "PrimitiveComponent Object Reference") (OtherBodyIndex :type Integer) (bFromSweep :type Boolean) (SweepResult :type "HitResult Structure (by ref)"))
  (bind _ascharacter (cast `Character` OtherActor))
  (if (and (not (`self.Open?`)) (`/CustomMapTools/Blueprints/BPFL_PavlovTemplate.IsPavPawn?` _ascharacter))
    (`self.ChangeDoorState` true)))

(event `ChangeDoorState`
  (params (State :type Boolean))
  (set `self.Open?` State))

(event `self.Box.OnComponentEndOverlap`
  (params (OverlappedComponent :type "PrimitiveComponent Object Reference") (OtherActor :type "Actor Object Reference") (OtherComp :type "PrimitiveComponent Object Reference") (OtherBodyIndex :type Integer))
  (cast `Character` OtherActor)
  (if (and (`self.Open?`) (< (`KismetArrayLibrary.Array_Length` (`PrimitiveComponent.GetOverlappingActors` (`self.Box`) "/Script/Engine.Character")) 1))
    (`self.ChangeDoorState` false)))

(event `Open Door`
  (bind _door (`self.Door`))
  ;[1 1 1] Open/Closes door from open? rep notify so the door is synced
  (bind (_direction _alpha) (`Timeline|MoveDoor` :!label _label)
    (:`Update`
      (if (`self.RotateOpen?`)
        (bind (_returnvalue_location _returnvalue_rotation) (`KismetMathLibrary.BreakTransform` (`KismetMathLibrary.TLerp` (`self.CloseTransform`) (`self.OpenTransform`) _alpha)))
        (`SceneComponent.K2_SetRelativeRotation` _door _returnvalue_rotation false false)
        (else
          (`SceneComponent.K2_SetRelativeLocation` _door _returnvalue_location false false))))))

(event `Close Door`
  ;[1 1 1] Open/Closes door from open? rep notify so the door is synced
  (goto _label :!via `Reverse`))

(fn `OnRep_Open?`
  (if (`self.Open?`)
    (`self.Open Door`)
    (else
      (`self.Close Door`))))

(fn `UserConstructionScript`
  (bind _arrow (`self.Arrow`))
  (if (`self.RotateOpen?`)
    (`SceneComponent.SetVisibility` _arrow true false)
    (else
      (`SceneComponent.SetVisibility` _arrow false false))))