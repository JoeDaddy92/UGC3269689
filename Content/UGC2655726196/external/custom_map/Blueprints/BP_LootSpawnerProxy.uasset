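; Placeable loot spawner proxy for custom maps that marks where weapons or equipment spawn, with its settings encoded as actor tags.
; The construction script rebuilds the tags from exposed variables: a LootSpawner marker, optional attachment stripping, a spawn-mode tag and item names.
; SpawnerType selects a zero-padded min/max timer, once-per-round spawning, or a fixed mode using only the first list item.
; It contains no runtime spawning logic.
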(fn `UserConstructionScript`
  (bind _minspawntime (`self.MinSpawnTime`))
  (bind _maxspawntime (`self.MaxSpawnTime`))
  (bind _tags (`self.Tags`))
  (`KismetArrayLibrary.Array_Clear` _tags)
  (`KismetArrayLibrary.Array_AddUnique` _tags "LootSpawner")
  (if (`self.SpawnWithoutAttachments`)
    (`KismetArrayLibrary.Array_AddUnique` _tags "StripWeapons"))
  (switch `int` (`self.SpawnerType`)
    (:`0`
      (`KismetArrayLibrary.Array_AddUnique` _tags (`KismetStringLibrary.Conv_StringToName` (`KismetStringLibrary.Concat_StrStr` "Time_" (select `bool` (> _minspawntime 9) :`false` (`KismetStringLibrary.Concat_StrStr` "00" (`KismetStringLibrary.Conv_IntToString` _minspawntime)) :`true` (select `bool` (> _minspawntime 99) :`false` (`KismetStringLibrary.Concat_StrStr` "0" (`KismetStringLibrary.Conv_IntToString` _minspawntime)) :`true` (`KismetStringLibrary.Conv_IntToString` _minspawntime))) "_" (select `bool` (> _maxspawntime 9) :`false` (`KismetStringLibrary.Concat_StrStr` "00" (`KismetStringLibrary.Conv_IntToString` _maxspawntime)) :`true` (select `bool` (> _maxspawntime 99) :`false` (`KismetStringLibrary.Concat_StrStr` "0" (`KismetStringLibrary.Conv_IntToString` _maxspawntime)) :`true` (`KismetStringLibrary.Conv_IntToString` _maxspawntime))))))
      (for _array_element (`self.SpawnList`) :!label _label
        (`KismetArrayLibrary.Array_Add` _tags (`KismetStringLibrary.Conv_StringToName` _array_element))))
    (:`1`
      (`KismetArrayLibrary.Array_AddUnique` _tags "Time_Rou")
      (goto _label))
    (:`2`
      (`KismetArrayLibrary.Array_AddUnique` _tags "Time_Non")
      (`KismetArrayLibrary.Array_AddUnique` _tags (`KismetStringLibrary.Conv_StringToName` (`|GetArrayItem` (`self.SpawnList`)))))))