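; Example Pavlov custom game mode logic and API reference, showing a timed match with repeating rounds.
; Server-side events set mode properties, start the match-end timer and drive round states with delays for cleanup, spawning, movement lock and buying.
; State changes are broadcast to all BPI_MatchRounds actors so they can react or reset.
; Spawns grant buy time and vitality; kill handling and team assignment are stubs, alongside unwired sample API calls.
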(event `self.OnCustomGameModeInit`
  ;[1 1 1] Init GameMode Properties when server starts
  ; Round duration will automatically handle the swap from roundstate started to ended
  (`self.SetGameModeProperties` (make `PavlovGameModeProperties` false true false 16000 300 3300 false true 5.0 false true 30 10 true true 30)))

(event `self.ReceiveBeginPlay`
  ;[1 1 1] Time till game starts EventOnRoundBegin will be triggered automatically when the match starts
  (`/Engine/EditorBlueprintResources/ActorMacros.Switch Has Authority`
    (:`Authority`
      (`self.Match Timer`))))

(event `self.OnPlayerJoinedServer`
  (params (PlayerStatus :type "PavlovPlayerStatus Structure (by ref)"))
  ;[1 1 1] Callback when players join/leave the server, If "Spawn Ghost On Login" is false then you need to handle connecting clients based on the Round State.
  ; If "Auto Respawn" & "Spawn Ghost On Login" are true then you need to handle incoming connections based on Round State(if the round state == started they will respawn)
)

(event `Play Sound FX 2D`
  (params (Sound :type "SoundBase Object Reference"))
  ;[1 1 1] Example of replicated 2d sound effect (make sure to call from server)
  ; Just an example, these calls will not work in this class
  (`GameplayStatics.PlaySound2D` Sound 1.0 1.0 0.0 null null))

(event `self.OnPlayerLeftServer`
  (params (PlayerStatus :type "PavlovPlayerStatus Structure (by ref)"))
  ;[1 1 1] Callback when players join/leave the server, If "Spawn Ghost On Login" is false then you need to handle connecting clients based on the Round State.
  ; If "Auto Respawn" & "Spawn Ghost On Login" are true then you need to handle incoming connections based on Round State(if the round state == started they will respawn)
)

(event `Play Sound FX At Location`
  (params (Sound :type "SoundBase Object Reference") (Location :type "Vector Structure"))
  ;[1 1 1] Example of replicated sound that plays at a location (use cues for attenuation, call from server) Just an example, these calls will not work in this class
  (`GameplayStatics.PlaySoundAtLocation` Sound Location (struct) 1.0 1.0 0.0 null null null null))

(event `self.OnRoundBegin`
  ;[1 1 1] This resets all players and cleans up all pavlov actors (you can use your own function to handle this if youd like)
  (`/Engine/EditorBlueprintResources/ActorMacros.Switch Has Authority`
    (:`Authority`
      (if (`self.FirstRound?`)
        (`KismetSystemLibrary.Delay` 7.0) ; Allows time for players to load in on first round
        (set `self.FirstRound?` false)
        (else
          (`KismetSystemLibrary.Delay` 1.0)))
      (`self.PostRoundCleanUp`)
      (`self.SpawnAndPosessPawns`)
      (`self.SetMovementDisabled` true)
      (`KismetSystemLibrary.Delay` 1.0)
      (for _array_element (`self.GetPlayers`)
        (`self.SetPlayerBuyingEnabled` _array_element 15.0 1000.0))
      (`self.SetRoundState` "StandBy")
      (`KismetSystemLibrary.Delay` 5.0) ; starting round buy time delay, need to have at least a 1 sec delay between changing round states
      (`self.SetRoundState` "Started")
      (`self.SetMovementDisabled` false))))

(event `self.OnRoundEnd`
  ;[1 1 1] Round End, change delays duration to adjust the wait for players to respawn and prepare before the match starts, must ensure there is at least a 1 sec delay between round state changes.
  (`/Engine/EditorBlueprintResources/ActorMacros.Switch Has Authority`
    (:`Authority`
      (`KismetSystemLibrary.PrintString` "Round End Declare Winner")
      (`KismetSystemLibrary.Delay` 2.0)
      (`self.SetRoundState` "Starting"))))

(event `Match Timer`
  ;[1 1 1] Time till match ends
  ; End match can be called due to specific requirements being met vs having it on a timer.
  (`KismetSystemLibrary.K2_SetTimerDelegate` (delegate `End Match`) 500.0))

(event `End Match`
  ;[1 1 1] Time till match ends
  ; End match can be called due to specific requirements being met vs having it on a timer.
  (`/Engine/EditorBlueprintResources/StandardMacros.DoOnce` false
    (:`Completed`
      (bind _asgame_mode (cast `GameMode` (`GameplayStatics.GetGameMode`)))
      (`GameMode.EndMatch` _asgame_mode))))

(event `self.OnRoundStateChanged`
  (params (OldState :type "EPavlovRoundState Enum" :default "Starting") (NewState :type "EPavlovRoundState Enum" :default "Starting"))
  ;[1 1 1] Updates all blueprints with BPI_MatchRounds implemented,
  ;  can be used to reset actors to initial state (This is covered in part 1 of the youtube series)
  (`self.RoundInterfaceCall` NewState)
  (`KismetSystemLibrary.PrintString` (`KismetStringLibrary.Concat_StrStr` (`|GetEnumeratorNameAsString` OldState) "||" (`|GetEnumeratorNameAsString` NewState))))

(event `self.OnPlayerKilled`
  (params (PlayerStatus :type "PavlovPlayerStatus Structure (by ref)") (Killer :type "PlayerState Object Reference") (bHeadshot :type Boolean) (KilledByItem :type Name))
  ;[1 1 1] All calls after EventOnPlayerKilled should be collapsed to a single function in order to prevent it from getting called twice and skipping the logic mid way through
  (bind (_alivepawns _alivecount) (`self.GetConnectedPawns`))
  (if (<= _alivecount 1)
    (bind _playerstatus (`PavlovProxyStatics.GetPavlovPlayerStatus` Killer))))

(event `self.OnPlayerSpawned`
  (params (PlayerStatus :type "PavlovPlayerStatus Structure (by ref)"))
  ;[1 1 1] Called when a player spawns in
  (`self.InitSpawnedPlayer` PlayerStatus))

(fn `GetConnectedPawns`
  (returns (AlivePawns :type "Array of Pawn Object Reference") (AliveCount :type Integer) (GhostPawns :type "Array of Pawn Object Reference") (GhostCount :type Integer))
  (locals (L_AliveCount :type Integer :default 0) (L_AlivePawns :type "Array of Pawn Object Reference") (L_GhostCount :type Integer) (L_GhostPawns :type "Array of Pawn Object Reference"))
  (for _array_element (`self.GetPlayers`)
    (bind (_playerstatus _bsucceeded) (`PavlovProxyStatics.GetPavlovPlayerStatus` _array_element))
    (if _bsucceeded
      (bind (_playerstate _controller _pawn) (break `PavlovPlayerStatus` _playerstatus))
      (if (`/CustomMapTools/Blueprints/BPFL_PavlovTemplate.IsPavPawn?` _pawn)
        (`/Engine/EditorBlueprintResources/StandardMacros.IncrementInt` (`local.L_AliveCount`)
          (:`  `
            (`KismetArrayLibrary.Array_AddUnique` (`local.L_AlivePawns`) _pawn)))
        (else
          (`/Engine/EditorBlueprintResources/StandardMacros.IncrementInt` (`local.L_GhostCount`)
            (:`  `
              (`KismetArrayLibrary.Array_AddUnique` (`local.L_GhostPawns`) _pawn)))))))
  (return (`local.L_AlivePawns`) (`local.L_AliveCount`) (`local.L_GhostPawns`) (`local.L_GhostCount`)))

(fn `GetPlayers`
  (returns (Players :type "Array of PlayerState Object Reference"))
  (bind _asgame_state (cast `GameState` (`GameplayStatics.GetGameState`)))
  (return (`GameStateBase.PlayerArray` _asgame_state)))

(fn `InitSpawnedPlayer`
  (params (PavlovPlayerStatus :type "PavlovPlayerStatus Structure (by ref)"))
  (bind _playerstate (break `PavlovPlayerStatus` PavlovPlayerStatus))
  (`self.SetPlayerBuyingEnabled` _playerstate 15.0 1000.0)
  (`self.SetPlayerVitality` _playerstate 100 100 1))

(fn `OnAssignTeam`
  (params (Status :type "PavlovPlayerStatus Structure (by ref)"))
  (returns (TeamId :type Integer))
  (if (> 0 0)
    (return 0)
    (else
      (return 1))))

(fn `RespawnPlayer`
  (params (PlayerStatus :type "PavlovPlayerStatus Structure (by ref)") (`As Ghost` :type Boolean) (`Spawn At Transform?` :type Boolean) (Transform :type "Transform Structure"))
  (bind (_playerstate _controller) (break `PavlovPlayerStatus` (`local.PlayerStatus`)))
  (if (`local.Spawn At Transform?`)
    (`self.Spawn` _controller (`local.Transform`) (`local.As Ghost`))
    (else
      (bind _transform (`self.GetSpawnTransform` _controller))
      (`self.Spawn` _controller _transform (`local.As Ghost`))))
  (return))

(fn `RoundInterfaceCall`
  (params (`Round State` :type "EPavlovRoundState Enum" :default "Starting"))
  (locals (L_InterfaceActors :type "Array of Actor Object Reference"))
  (bind _l_interfaceactors (`local.L_InterfaceActors`))
  (bind _outactors (`GameplayStatics.GetAllActorsWithInterface` "/CustomMapTools/Blueprints/BPI_MatchRounds.BPI_MatchRounds_C"))
  (set `local.L_InterfaceActors` _outactors)
  (switch `EPavlovRoundState` (`local.Round State`)
    (:`Starting`
      (message `/CustomMapTools/Blueprints/BPI_MatchRounds.RoundStarting` _l_interfaceactors))
    (:`StandBy`
      (message `/CustomMapTools/Blueprints/BPI_MatchRounds.RoundStandBy` _l_interfaceactors))
    (:`Started`
      (message `/CustomMapTools/Blueprints/BPI_MatchRounds.RoundStarted` _l_interfaceactors))
    (:`Ended`
      (message `/CustomMapTools/Blueprints/BPI_MatchRounds.RoundEnded` _l_interfaceactors)))
  (return))

(fn `UserConstructionScript`)